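; BP_MenuPrincipal is a main menu Blueprint that continuously spins its Capsule component around the yaw axis.
; On BeginPlay it caches the capsule's world rotation, then a timeline lerps a yaw offset from 0 to 360 degrees while keeping pitch and roll.
; The timeline restarts on finish for an endless loop, setting relative rotation during updates but world rotation at each finish.
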(event `self.ReceiveBeginPlay`
  (bind (_initialrotation_roll _initialrotation_pitch _initialrotation_yaw) (`KismetMathLibrary.BreakRotator` (`self.InitialRotation`)))
  (set `self.InitialRotation` (`SceneComponent.K2_GetComponentRotation` (`self.Capsule`)))
  (bind (_direction _newtrack_0) (`Timeline|RotateTL` :!via `PlayFromStart` :!label _label)
    (:`Update`
      (bind _returnvalue (+ _initialrotation_yaw (`KismetMathLibrary.Lerp` 0.0 360.0 _newtrack_0)))
      (`SceneComponent.K2_SetRelativeRotation` (`self.Capsule`) (`KismetMathLibrary.MakeRotator` _initialrotation_roll _initialrotation_pitch _returnvalue) false false))
    (:`Finished`
      (`SceneComponent.K2_SetWorldRotation` (`self.Capsule`) (`KismetMathLibrary.MakeRotator` _initialrotation_roll _initialrotation_pitch _returnvalue) false false)
      (goto _label :!via `PlayFromStart`))))

(fn `UserConstructionScript`)