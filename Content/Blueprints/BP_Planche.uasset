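; BP_Planche is a pushable plank that the player shoves along rounded forward directions by walking into it.
; On hit it freezes and attaches the player, then a timeline slides it by TravelDistance, repeating while Z or Q is held.
; Releasing restores walking and calls detach on the plank itself, not the player.
; Its Box overlapping a BP_PlancheStop ends pushing and permanently clears CanInteract.
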(event `self.ReceiveBeginPlay`)

(event `self.ReceiveHit`
  (params (MyComp :type "PrimitiveComponent Object Reference") (Other :type "Actor Object Reference") (OtherComp :type "PrimitiveComponent Object Reference") (bSelfMoved :type Boolean) (HitLocation :type "Vector Structure") (HitNormal :type "Vector Structure") (NormalImpulse :type "Vector Structure") (Hit :type "HitResult Structure (by ref)"))
  (bind _returnvalue (`GameplayStatics.GetPlayerCharacter` 0))
  (if (== (`GameplayStatics.GetPlayerCharacter` 0) Other)
    (if (`self.CanInteract`)
      (set `self.PushDirection` (`KismetMathLibrary.MakeVector` (`KismetMathLibrary.Conv_IntToDouble` (`KismetMathLibrary.Round` (.x (`self.GetActorForwardVector` Other)))) (`KismetMathLibrary.Conv_IntToDouble` (`KismetMathLibrary.Round` (.y (`self.GetActorForwardVector` Other)))) (`KismetMathLibrary.Conv_IntToDouble` (`KismetMathLibrary.Round` (.z (`self.GetActorForwardVector` Other))))))
      (`CharacterMovementComponent.DisableMovement` (`Character.CharacterMovement` _returnvalue))
      (`self.K2_AttachToActor` _returnvalue self "None" "KeepWorld" "KeepWorld" "KeepWorld" true)
      (`self.Push`))))

(event `Push`
  (if (`self.CanInteract`)
    (set `self.CurrentLocation` (`self.K2_GetActorLocation`))
    (bind (_direction _newtrack_0) (`Timeline|MoveBlock` :!via `PlayFromStart`)
      (:`Update`
        (`self.K2_SetActorRelativeLocation` (+ (`self.CurrentLocation`) (* _newtrack_0 (`self.PushDirection`) (`self.TravelDistance`)))))
      (:`Finished`
        (if (`PlayerController.IsInputKeyDown` (`GameplayStatics.GetPlayerController` 0) "Z")
          (`self.Push`)
          (elif (`PlayerController.IsInputKeyDown` (`GameplayStatics.GetPlayerController` 0) "Q")
            (`self.Push`)
            (elif (`PlayerController.IsInputKeyDown` (`GameplayStatics.GetPlayerController` 0) "Q")
              (`self.Push`)
              (else
                (`self.StopPushing`)))))))))

(event `StopPushing`
  (`CharacterMovementComponent.SetMovementMode` (`Character.CharacterMovement` (`GameplayStatics.GetPlayerCharacter` 0)) "MOVE_Walking" 0)
  (`self.K2_DetachFromActor` "KeepWorld" "KeepWorld" "KeepWorld"))

(event `self.Box.OnComponentBeginOverlap`
  (params (OverlappedComponent :type "PrimitiveComponent Object Reference") (OtherActor :type "Actor Object Reference") (OtherComp :type "PrimitiveComponent Object Reference") (OtherBodyIndex :type Integer) (bFromSweep :type Boolean) (SweepResult :type "HitResult Structure (by ref)"))
  (cast `/Game/Blueprints/BP_PlancheStop` OtherActor)
  (set `self.CanInteract` false)
  (`self.StopPushing`))

(fn `UserConstructionScript`)