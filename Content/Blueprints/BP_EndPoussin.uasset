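; BP_EndPoussin plays an ending camera sequence that leads into the credits.
; On BeginPlay, a timeline moves and rotates the camera along Spline1 by scaling one track against the spline's length.
; A second track fades a camera post-process value down to zero through a lerp.
; When the timeline finishes, it creates the WB_Credits widget and adds it to the viewport.
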(event `self.ReceiveBeginPlay`
  (bind _spline1 (`self.Spline1`))
  (bind _camera (`self.Camera`))
  (bind (_direction _newtrack_0 _newtrack_1) (`Timeline|Timeline` :!via `PlayFromStart`)
    (:`Update`
      (bind _returnvalue (* _newtrack_1 (`SplineComponent.GetSplineLength` _spline1)))
      (`SceneComponent.K2_SetWorldLocation` _camera (`SplineComponent.GetLocationAtDistanceAlongSpline` _spline1 _returnvalue "World") false false)
      (`SceneComponent.K2_SetWorldRotation` _camera (`SplineComponent.GetRotationAtDistanceAlongSpline` _spline1 _returnvalue "World") false false)
      (set `CameraComponent.PostProcessSettings` (make `PostProcessSettings` :`VignetteIntensity` (`KismetMathLibrary.Lerp` 200.0 0.0 _newtrack_0)) (`self.Camera`)))
    (:`Finished`
      (bind _returnvalue_2 (`|CreateWidget` "/Game/Widgets/WB_Credits.WB_Credits_C"))
      (`UserWidget.AddToViewport` _returnvalue_2 0))))

(fn `UserConstructionScript`)