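; BP_PotionPossess is a possess potion actor that unlocks the CanAddPoussin ability flag when the player touches it.
; On BeginPlay it applies the MI_PotionPossess material to its Cylinder, then calls the parent's BeginPlay.
; A Box overlap by player character 0 sets CanAddPoussin on GMRef, guarded by a DoOnce so it fires only once.
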(event `self.ReceiveBeginPlay`
  (`PrimitiveComponent.SetMaterial` (`self.Cylinder`) 0 "/Game/Materials/MI_PotionPossess.MI_PotionPossess")
  (`parent.ReceiveBeginPlay`))

(event `self.Box.OnComponentBeginOverlap`
  (params (OverlappedComponent :type "PrimitiveComponent Object Reference") (OtherActor :type "Actor Object Reference") (OtherComp :type "PrimitiveComponent Object Reference") (OtherBodyIndex :type Integer) (bFromSweep :type Boolean) (SweepResult :type "HitResult Structure (by ref)"))
  (if (== OtherActor (`GameplayStatics.GetPlayerCharacter` 0))
    (`/Engine/EditorBlueprintResources/StandardMacros.DoOnce` false
      (:`Completed`
        (set `/Game/ThirdPerson/Blueprints/BP_ThirdPersonGameMode.CanAddPoussin?` true (`self.GMRef`))))))

(fn `UserConstructionScript`
  (`parent.UserConstructionScript`))