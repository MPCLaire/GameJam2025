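; BP_PotionForce is a strength potion pickup that grants the player the ability to push.
; It extends a parent Blueprint, applying the MI_PotionForce material to its Fiole component on BeginPlay.
; The first player overlap with its Box sets CanPush on GMRef and activates the Drink component.
; It then spawns a BP_ParticlesPotion below the player's location, sets its color and attaches it to the player.
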(event `self.ReceiveBeginPlay`
  (`PrimitiveComponent.SetMaterial` (`self.Fiole`) 0 "/Game/Materials/MI_PotionForce.MI_PotionForce")
  (`parent.ReceiveBeginPlay`))

(event `self.Box.OnComponentBeginOverlap`
  (params (OverlappedComponent :type "PrimitiveComponent Object Reference") (OtherActor :type "Actor Object Reference") (OtherComp :type "PrimitiveComponent Object Reference") (OtherBodyIndex :type Integer) (bFromSweep :type Boolean) (SweepResult :type "HitResult Structure (by ref)"))
  (bind _returnvalue (`GameplayStatics.GetPlayerCharacter` 0))
  (bind (_returnvalue_x _returnvalue_y _returnvalue_z) (`KismetMathLibrary.BreakVector` (`self.K2_GetActorLocation` _returnvalue)))
  (if (== OtherActor _returnvalue)
    (`/Engine/EditorBlueprintResources/StandardMacros.DoOnce` false
      (:`Completed`
        (set `/Game/ThirdPerson/Blueprints/BP_ThirdPersonGameMode.CanPush?` true (`self.GMRef`))
        (`ActorComponent.Activate` (`self.Drink`) false)
        (bind _returnvalue_2 (`|SpawnActorFromClass` "/Game/Blueprints/BP_ParticlesPotion.BP_ParticlesPotion_C" (`KismetMathLibrary.MakeTransform` (`KismetMathLibrary.MakeVector` _returnvalue_x _returnvalue_y (- _returnvalue_z 45.0))) "AlwaysSpawn" "MultiplyWithRoot" null null))
        (`/Game/Blueprints/BP_ParticlesPotion.SetParticleColor` _returnvalue_2 1)
        (`self.K2_AttachToActor` _returnvalue_2 _returnvalue "None" "KeepWorld" "KeepWorld" "KeepWorld" true)))))

(fn `UserConstructionScript`
  (`parent.UserConstructionScript`))