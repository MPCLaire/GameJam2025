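; BP_Cage is a cage whose door opens when the third-person character enters its Box trigger.
; The overlap turns on physics for the latch (Loquet) and knocks it loose with an impulse, then after a short delay calls OpenDoor.
; OpenDoor uses a timeline to swing the Pivot's yaw from its starting rotation.
; Latch physics is switched off again shortly after.
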(event `self.Box.OnComponentBeginOverlap`
  (params (OverlappedComponent :type "PrimitiveComponent Object Reference") (OtherActor :type "Actor Object Reference") (OtherComp :type "PrimitiveComponent Object Reference") (OtherBodyIndex :type Integer) (bFromSweep :type Boolean) (SweepResult :type "HitResult Structure (by ref)"))
  (bind _loquet (`self.Loquet`))
  (cast `/Game/ThirdPerson/Blueprints/BP_ThirdPersonCharacter` OtherActor)
  (`PrimitiveComponent.SetSimulatePhysics` _loquet true)
  (`PrimitiveComponent.AddImpulse` _loquet (0.0 200.0 200.0) "None" false)
  (`KismetSystemLibrary.Delay` 0.5)
  (`self.OpenDoor`)
  (`KismetSystemLibrary.Delay` 2.0)
  (`PrimitiveComponent.SetSimulatePhysics` (`self.Loquet`) false))

(event `OpenDoor`
  (bind (_initialrotation_roll _initialrotation_pitch _initialrotation_yaw) (`KismetMathLibrary.BreakRotator` (`self.InitialRotation`)))
  (set `self.InitialRotation` (`SceneComponent.K2_GetComponentRotation` (`self.Pivot`)))
  (bind (_direction _newtrack_0) (`Timeline|OpenDoorTL` :!via `PlayFromStart`)
    (:`Update`
      (`SceneComponent.K2_SetWorldRotation` (`self.Pivot`) (`KismetMathLibrary.MakeRotator` _initialrotation_roll _initialrotation_pitch (+ _initialrotation_yaw (`KismetMathLibrary.Lerp` 0.0 120.0 _newtrack_0))) false false))))

(fn `UserConstructionScript`)