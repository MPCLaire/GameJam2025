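; Elevator actor (Ascenseur) that moves its Cube in two trigger-driven stages, horizontal then vertical.
; The first Box overlap plays a one-shot Timeline that slides the Cube along negative Y and sets HasMove when finished.
; Once HasMove is set, entering VerticalBox stores the Cube's location and raises it on Z through a second Timeline, which reverses on exit.
; Both lerps start from zero rather than the stored position, and neither trigger filters the overlapping actor.
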(event `self.ReceiveBeginPlay`)

(event `self.Box.OnComponentBeginOverlap`
  (params (OverlappedComponent :type "PrimitiveComponent Object Reference") (OtherActor :type "Actor Object Reference") (OtherComp :type "PrimitiveComponent Object Reference") (OtherBodyIndex :type Integer) (bFromSweep :type Boolean) (SweepResult :type "HitResult Structure (by ref)"))
  (bind (_location_x _location_y _location_z) (`KismetMathLibrary.BreakVector` (`self.Location`)))
  (set `self.Location` (`SceneComponent.RelativeLocation` (`self.Cube`)))
  (`/Engine/EditorBlueprintResources/StandardMacros.DoOnce` false
    (:`Completed`
      (bind (_direction _newtrack_0) (`Timeline|Timeline`)
        (:`Update`
          (`SceneComponent.K2_SetRelativeLocation` (`self.Cube`) (`KismetMathLibrary.MakeVector` _location_x (`KismetMathLibrary.Lerp` 0.0 (+ _location_y -330.0) _newtrack_0) _location_z) false false))
        (:`Finished`
          (set `self.HasMove` true))))))

(event `self.VerticalBox.OnComponentBeginOverlap`
  (params (OverlappedComponent :type "PrimitiveComponent Object Reference") (OtherActor :type "Actor Object Reference") (OtherComp :type "PrimitiveComponent Object Reference") (OtherBodyIndex :type Integer) (bFromSweep :type Boolean) (SweepResult :type "HitResult Structure (by ref)"))
  (bind (_location_x _location_y _location_z) (`KismetMathLibrary.BreakVector` (`self.Location`)))
  (if (`self.HasMove`)
    (set `self.Location` (`SceneComponent.RelativeLocation` (`self.Cube`)))
    (bind (_direction _newtrack_0) (`Timeline|Timeline_0` :!label _label)
      (:`Update`
        (`SceneComponent.K2_SetRelativeLocation` (`self.Cube`) (`KismetMathLibrary.MakeVector` _location_x _location_y (`KismetMathLibrary.Lerp` 0.0 (+ _location_z 200.0) _newtrack_0)) false false)))))

(event `self.VerticalBox.OnComponentEndOverlap`
  (params (OverlappedComponent :type "PrimitiveComponent Object Reference") (OtherActor :type "Actor Object Reference") (OtherComp :type "PrimitiveComponent Object Reference") (OtherBodyIndex :type Integer))
  (goto _label :!via `Reverse`))

(fn `UserConstructionScript`)