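; BP_PressurePlate1 is a pressure plate that controls a referenced door when the player steps on or off it.
; Overlap begin and end events on its Collision component, filtered by the "player" tag, each call SwitchOnOff on DoorRef1.
; The PressurePlate timeline plays on entry and reverses on exit, lerping the Plate's relative Z location so it sinks slightly and rises back.
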(event `self.Collision.OnComponentBeginOverlap`
  (params (OverlappedComponent :type "PrimitiveComponent Object Reference") (OtherActor :type "Actor Object Reference") (OtherComp :type "PrimitiveComponent Object Reference") (OtherBodyIndex :type Integer) (bFromSweep :type Boolean) (SweepResult :type "HitResult Structure (by ref)"))
  (if (`self.ActorHasTag` OtherActor "player")
    (`/Game/BP_Door1.SwitchOnOff` (`self.DoorRef1`))
    (bind (_direction _newtrack_0) (`Timeline|PressurePlate` :!label _label)
      (:`Update`
        (`SceneComponent.K2_SetRelativeLocation` (`self.Plate`) (`KismetMathLibrary.MakeVector` 0.0 0.0 (`KismetMathLibrary.Lerp` 0.0 -5.0 _newtrack_0)) false false)))))

(event `self.Collision.OnComponentEndOverlap`
  (params (OverlappedComponent :type "PrimitiveComponent Object Reference") (OtherActor :type "Actor Object Reference") (OtherComp :type "PrimitiveComponent Object Reference") (OtherBodyIndex :type Integer))
  (if (`self.ActorHasTag` OtherActor "player")
    (`/Game/BP_Door1.SwitchOnOff` (`self.DoorRef1`))
    (goto _label :!via `Reverse`)))

(fn `UserConstructionScript`)